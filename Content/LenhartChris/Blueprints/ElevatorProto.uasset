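; Prototype elevator actor that lifts its pad when a character steps into its trigger box.
; Box overlap plays a timeline that lerps ElevatorPad's relative location straight up along Z.
; When the character leaves the box, a short delay precedes reversing the timeline to lower the pad.
; Characters are identified by checking whether the overlapping actor's display name contains "character", rather than by casting.
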(event `self.Box.OnComponentBeginOverlap`
  (params (OverlappedComponent :type "PrimitiveComponent Object Reference") (OtherActor :type "Actor Object Reference") (OtherComp :type "PrimitiveComponent Object Reference") (OtherBodyIndex :type Integer) (bFromSweep :type Boolean) (SweepResult :type "HitResult Structure (by ref)"))
  ;[1 1 1] Elevator Code
  (if (`KismetStringLibrary.Contains` (`KismetSystemLibrary.GetDisplayName` OtherActor) "character")
    (bind (_direction _newtrack_0) (`Timeline|Timeline_0` :!label _label)
      (:`Update`
        (`SceneComponent.K2_SetRelativeLocation` (`self.ElevatorPad`) (`KismetMathLibrary.VLerp` (0.0 0.0 0.0) (0.0 0.0 1150.0) _newtrack_0) false false)))))

(event `self.Box.OnComponentEndOverlap`
  (params (OverlappedComponent :type "PrimitiveComponent Object Reference") (OtherActor :type "Actor Object Reference") (OtherComp :type "PrimitiveComponent Object Reference") (OtherBodyIndex :type Integer))
  ;[1 1 1] Elevator Code
  (if (`KismetStringLibrary.Contains` (`KismetSystemLibrary.GetDisplayName` OtherActor) "character")
    (`KismetSystemLibrary.Delay` 1.5)
    (goto _label :!via `Reverse`)))

(fn `UserConstructionScript`)
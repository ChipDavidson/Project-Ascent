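; A sliding double door Blueprint that opens when a character enters its Front trigger and closes after they leave.
; The OpenDoor timeline lerps Left, Right, Top and Bottom panels outward from the center, identifying characters by "character" in the display name.
; On exit, a short delay precedes reversing the timeline.
; The pending close is not cancelled on re-entry, so the door can close on a returning character.
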(event `self.Front.OnComponentBeginOverlap`
  (params (OverlappedComponent :type "PrimitiveComponent Object Reference") (OtherActor :type "Actor Object Reference") (OtherComp :type "PrimitiveComponent Object Reference") (OtherBodyIndex :type Integer) (bFromSweep :type Boolean) (SweepResult :type "HitResult Structure (by ref)"))
  ;[1 1 1] Double Door Works, but when player leaves itll close again even if player steps in really fast
  (if (`KismetStringLibrary.Contains` (`KismetSystemLibrary.GetDisplayName` OtherActor) "character")
    (bind (_direction _newtrack_0) (`Timeline|Open Door` :!label _label)
      (:`Update`
        (`SceneComponent.K2_SetRelativeLocation` (`self.Left`) (`KismetMathLibrary.VLerp` (-105.003586 0.0 69.003593) (-305.003601 0.0 69.003593) _newtrack_0) false false)
        (`SceneComponent.K2_SetRelativeLocation` (`self.Right`) (`KismetMathLibrary.VLerp` (106.996414 0.0 69.003593) (306.996399 0.0 69.003593) _newtrack_0) false false)
        (`SceneComponent.K2_SetRelativeLocation` (`self.Top`) (`KismetMathLibrary.VLerp` (0.996414 0.0 175.003601) (0.996414 0.0 375.003601) _newtrack_0) false false)
        (`SceneComponent.K2_SetRelativeLocation` (`self.Bottom`) (`KismetMathLibrary.VLerp` (0.996414 0.0 -36.996399) (0.996414 0.0 -236.996399) _newtrack_0) false false)))))

(event `self.Front.OnComponentEndOverlap`
  (params (OverlappedComponent :type "PrimitiveComponent Object Reference") (OtherActor :type "Actor Object Reference") (OtherComp :type "PrimitiveComponent Object Reference") (OtherBodyIndex :type Integer))
  ;[1 1 1] Double Door Works, but when player leaves itll close again even if player steps in really fast
  (if (`KismetStringLibrary.Contains` (`KismetSystemLibrary.GetDisplayName` OtherActor) "character")
    (`KismetSystemLibrary.Delay` 2.0)
    (goto _label :!via `Reverse`)))

(fn `UserConstructionScript`)
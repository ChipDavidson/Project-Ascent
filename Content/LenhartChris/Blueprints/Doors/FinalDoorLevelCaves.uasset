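; One-way final door for the caves level that opens when a character enters its front collision.
; The overlap checks the actor's display name for "character", then a DoOnce with no reset plays a timeline.
; Each update nudges the top pieces up and the bottom crystals down, lerping from their current relative location, so movement accumulates rather than following fixed endpoints.
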(event `self.FrontDoorCollision.OnComponentBeginOverlap`
  (params (OverlappedComponent :type "PrimitiveComponent Object Reference") (OtherActor :type "Actor Object Reference") (OtherComp :type "PrimitiveComponent Object Reference") (OtherBodyIndex :type Integer) (bFromSweep :type Boolean) (SweepResult :type "HitResult Structure (by ref)"))
  (bind _crystal (`self.Crystal`))
  (bind _crystal1 (`self.Crystal1`))
  (bind _crystal7 (`self.Crystal7`))
  (bind _crystal8 (`self.Crystal8`))
  (bind _crystal2 (`self.Crystal2`))
  (bind _top (`self.Top`))
  (bind _top1 (`self.Top1`))
  (bind _top2 (`self.Top2`))
  (bind _top3 (`self.Top3`))
  (bind _top4 (`self.Top4`))
  (bind _top5 (`self.Top5`))
  (bind _relativelocation (`SceneComponent.RelativeLocation` _top5))
  (bind _relativelocation_2 (`SceneComponent.RelativeLocation` _top2))
  (bind _relativelocation_3 (`SceneComponent.RelativeLocation` _top))
  (bind _relativelocation_4 (`SceneComponent.RelativeLocation` _top1))
  (bind _relativelocation_5 (`SceneComponent.RelativeLocation` _top3))
  (bind _relativelocation_6 (`SceneComponent.RelativeLocation` _crystal))
  (bind _relativelocation_7 (`SceneComponent.RelativeLocation` _crystal1))
  (bind _relativelocation_8 (`SceneComponent.RelativeLocation` _crystal7))
  (bind _relativelocation_9 (`SceneComponent.RelativeLocation` _crystal8))
  (bind _relativelocation_10 (`SceneComponent.RelativeLocation` _crystal2))
  (bind _relativelocation_11 (`SceneComponent.RelativeLocation` _top4))
  ;[1 1 1] One Way Door Works
  (if (`KismetStringLibrary.Contains` (`KismetSystemLibrary.GetDisplayName` OtherActor) "character")
    (`/Engine/EditorBlueprintResources/StandardMacros.DoOnce` false
      (:`Completed`
        (bind (_direction _newtrack_0) (`Timeline|Timeline_0`)
          (:`Update`
            ;;[1 1 1] Top
            (`SceneComponent.K2_SetRelativeLocation` _top (`KismetMathLibrary.VLerp` _relativelocation_3 (+ _relativelocation_3 (0.0 0.0 4.0)) _newtrack_0) false false)
            (`SceneComponent.K2_SetRelativeLocation` _top1 (`KismetMathLibrary.VLerp` _relativelocation_4 (+ _relativelocation_4 (0.0 0.0 4.0)) _newtrack_0) false false)
            (`SceneComponent.K2_SetRelativeLocation` _top2 (`KismetMathLibrary.VLerp` _relativelocation_2 (+ _relativelocation_2 (0.0 0.0 4.0)) _newtrack_0) false false)
            (`SceneComponent.K2_SetRelativeLocation` _top3 (`KismetMathLibrary.VLerp` _relativelocation_5 (+ _relativelocation_5 (0.0 0.0 4.0)) _newtrack_0) false false)
            (`SceneComponent.K2_SetRelativeLocation` _top4 (`KismetMathLibrary.VLerp` _relativelocation_11 (+ _relativelocation_11 (0.0 0.0 4.0)) _newtrack_0) false false)
            (`SceneComponent.K2_SetRelativeLocation` _top5 (`KismetMathLibrary.VLerp` _relativelocation (+ _relativelocation (0.0 0.0 4.0)) _newtrack_0) false false)
            ;;[1 1 1] Bottom
            (`SceneComponent.K2_SetRelativeLocation` _crystal (`KismetMathLibrary.VLerp` _relativelocation_6 (+ _relativelocation_6 (0.0 0.0 -12.0)) _newtrack_0) false false)
            (`SceneComponent.K2_SetRelativeLocation` _crystal1 (`KismetMathLibrary.VLerp` _relativelocation_7 (+ _relativelocation_7 (0.0 0.0 -12.0)) _newtrack_0) false false)
            (`SceneComponent.K2_SetRelativeLocation` _crystal7 (`KismetMathLibrary.VLerp` _relativelocation_8 (+ _relativelocation_8 (0.0 0.0 -12.0)) _newtrack_0) false false)
            (`SceneComponent.K2_SetRelativeLocation` _crystal8 (`KismetMathLibrary.VLerp` _relativelocation_9 (+ _relativelocation_9 (0.0 0.0 -12.0)) _newtrack_0) false false)
            (`SceneComponent.K2_SetRelativeLocation` _crystal2 (`KismetMathLibrary.VLerp` _relativelocation_10 (+ _relativelocation_10 (0.0 0.0 -12.0)) _newtrack_0) false false)))))))

(fn `UserConstructionScript`)
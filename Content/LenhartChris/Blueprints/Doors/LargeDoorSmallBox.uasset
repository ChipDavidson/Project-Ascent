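; Large door Blueprint that opens in four panels when an actor with "character" in its display name enters its box trigger.
; The OpenDoor timeline pushes the left, right, top and bottom panels outward, and leaving the box reverses it after a delay.
; Each update lerps from the panel's current location, so movement accumulates and reversing does not itself restore the closed positions.
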(event `self.Box.OnComponentBeginOverlap`
  (params (OverlappedComponent :type "PrimitiveComponent Object Reference") (OtherActor :type "Actor Object Reference") (OtherComp :type "PrimitiveComponent Object Reference") (OtherBodyIndex :type Integer) (bFromSweep :type Boolean) (SweepResult :type "HitResult Structure (by ref)"))
  (bind _left (`self.Left`))
  (bind _right (`self.Right`))
  (bind _top (`self.Top`))
  (bind _bottom (`self.Bottom`))
  (bind _relativelocation (`SceneComponent.RelativeLocation` _left))
  (bind _relativelocation_2 (`SceneComponent.RelativeLocation` _right))
  (bind _relativelocation_3 (`SceneComponent.RelativeLocation` _top))
  (bind _relativelocation_4 (`SceneComponent.RelativeLocation` _bottom))
  ;[1 1 1] One Way Door Works
  (if (`KismetStringLibrary.Contains` (`KismetSystemLibrary.GetDisplayName` OtherActor) "character")
    (bind (_direction _newtrack_0) (`Timeline|Open Door` :!label _label)
      (:`Update`
        (`SceneComponent.K2_SetRelativeLocation` _left (`KismetMathLibrary.VLerp` _relativelocation (+ _relativelocation (-5.0 0.0 0.0)) _newtrack_0) false false)
        (`SceneComponent.K2_SetRelativeLocation` _right (`KismetMathLibrary.VLerp` _relativelocation_2 (+ _relativelocation_2 (5.0 0.0 0.0)) _newtrack_0) false false)
        (`SceneComponent.K2_SetRelativeLocation` _top (`KismetMathLibrary.VLerp` _relativelocation_3 (+ _relativelocation_3 (0.0 0.0 5.0)) _newtrack_0) false false)
        (`SceneComponent.K2_SetRelativeLocation` _bottom (`KismetMathLibrary.VLerp` _relativelocation_4 (+ _relativelocation_4 (0.0 0.0 -5.0)) _newtrack_0) false false)))))

(event `self.Box.OnComponentEndOverlap`
  (params (OverlappedComponent :type "PrimitiveComponent Object Reference") (OtherActor :type "Actor Object Reference") (OtherComp :type "PrimitiveComponent Object Reference") (OtherBodyIndex :type Integer))
  ;[1 1 1] One Way Door Works
  (if (`KismetStringLibrary.Contains` (`KismetSystemLibrary.GetDisplayName` OtherActor) "character")
    (`KismetSystemLibrary.Delay` 3.0)
    (goto _label :!via `Reverse`)))

(fn `UserConstructionScript`)
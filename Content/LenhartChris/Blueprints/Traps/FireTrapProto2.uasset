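; A prototype fire trap that moves along a path and teleports characters who touch it back to a respawn location.
; The construction script feeds two relative points (L1, L2) and a Duration into an InterpToMovement component.
; FireBox overlap finds characters by matching "Character" in the actor's display name, then moves them to PlayerRespawn.
; An unconnected cast-based respawn branch and an unused vector lerp remain in the graph.
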(event `self.FireBox.OnComponentBeginOverlap`
  (params (OverlappedComponent :type "PrimitiveComponent Object Reference") (OtherActor :type "Actor Object Reference") (OtherComp :type "PrimitiveComponent Object Reference") (OtherBodyIndex :type Integer) (bFromSweep :type Boolean) (SweepResult :type "HitResult Structure (by ref)"))
  ;[1 1 1] Respawning After Collision
  (if (`KismetStringLibrary.Contains` (`KismetSystemLibrary.GetDisplayName` OtherActor) "Character")
    (`self.K2_SetActorLocation` OtherActor (`self.PlayerRespawn`) false false)))

(fn `UserConstructionScript`
  (bind _interptomovement (`self.InterpToMovement`))
  (set `InterpToMovementComponent.ControlPoints` (`|MakeArray` (make `InterpControlPoint` (`self.L1`)) (make `InterpControlPoint` (`self.L2`))) _interptomovement)
  (set `InterpToMovementComponent.Duration` (`self.Duration`) _interptomovement))
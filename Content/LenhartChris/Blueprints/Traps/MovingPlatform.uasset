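; MovingPlatform is a trap Blueprint for a platform that moves between two configurable locations.
; Its construction script feeds L1 and L2 into an InterpToMovement component as relative control points and sets the travel time from the Duration variable.
; The event graph holds only unreachable respawn logic, noted as not working, that would teleport to PlayerRespawn after a name check for "Character".
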(fn `UserConstructionScript`
  (bind _interptomovement (`self.InterpToMovement`))
  ;[1 1 1] Movement between two locations , able to adjust time too with green float
  (set `InterpToMovementComponent.ControlPoints` (`|MakeArray` (make `InterpControlPoint` (`self.L1`)) (make `InterpControlPoint` (`self.L2`))) _interptomovement)
  (set `InterpToMovementComponent.Duration` (`self.Duration`) _interptomovement))